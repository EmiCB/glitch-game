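; BP_Glitch is a game mode Blueprint that runs an in-game clock and adds a Timer widget to the viewport on BeginPlay.
; A Delay on Tick paces the clock to advance one minute every five seconds, rolling minutes over into hours.
; When the hour count reaches twelve, it casts the player pawn to BP_Player and calls CheckIfDead with true.
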(event EventBeginPlay
  (bind _returnvalue (UserInterface|CreateWidget "/Game/Glitch/Player/HUD_Widgets/Timer.Timer_C"))
  (UserInterface|Viewport|AddtoViewport _returnvalue 0))

(event EventTick
  (params (DeltaSeconds :type Float%20%28single-precision%29))
  (Utilities|FlowControl|Delay 5.0)
  (if (== (Variables|Default|GetMinutes) 59)
    (Variables|Default|SetMinutes 0)
    (Variables|Default|SetHours (+ (Variables|Default|GetHours) 1))
    (if (== (Variables|Default|GetHours) 12)
      (bind _asbp_player (Utilities|Casting|CastToBP_Player (Game|Player|GetPlayerPawn 0)))
      (Default|CheckifDead _asbp_player true))
    (else
      (Variables|Default|SetMinutes (+ (Variables|Default|GetMinutes) 1)))))

(fn ConstructionScript)