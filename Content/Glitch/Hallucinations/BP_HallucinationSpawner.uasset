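; BP_HallucinationSpawner is an actor that triggers random hallucinations at intervals during play.
; On BeginPlay it caches door, bed and radio references, with the radio lookup nested inside the bed loop.
; A Delay on Tick acts as a repeating random timer of roughly a minute, then GenerateRandomEvent picks one of four events.
; Each skips if already active: glitch door, bed, radio, or an organ spawned at a fixed transform alongside old TVs switching on.
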(event EventBeginPlay
  (bind _outactors (Actor|GetAllActorsOfClass "/Game/Glitch/Furniture/Door/GlitchDoor.GlitchDoor_C"))
  (for _array_element _outactors
    (Variables|Default|SetDoorRef _array_element))
  (bind _outactors_2 (Actor|GetAllActorsOfClass "/Game/Glitch/Furniture/Bed/Bed.Bed_C"))
  (for _array_element_2 _outactors_2
    (Variables|Default|SetBed%20Ref _array_element_2)
    (bind _outactors_3 (Actor|GetAllActorsOfClass "/Game/HorrorEngine/Blueprints/UsableAssets/Electronics/Radio.Radio_C"))
    (for _array_element_3 _outactors_3
      (Variables|Default|SetRadio%20Ref _array_element_3))))

(event EventTick
  (params (DeltaSeconds :type Float%20%28single-precision%29))
  (bind _bed_ref (Variables|Default|GetBed%20Ref))
  (bind _doorref (Variables|Default|GetDoorRef))
  (bind _radio_ref (Variables|Default|GetRadio%20Ref))
  (Utilities|FlowControl|Delay (Math|Conversions|ToFloat(Integer) (Math|Random|RandomIntegerinRange 50 75)))
  (CallFunction|GenerateRandomEvent 4)
  (Development|PrintString "Exec Hallucination")
  (switch int (Variables|Default|GetCurrentEvent)
    (:0
      (if (not (Variables|/Game/Glitch/Furniture/Door/GlitchDoor.GlitchDoor_C|GetIsHallucinationStarted _doorref))
        (Default|StartHallucination _doorref)))
    (:1
      (if (not (Variables|/Game/Glitch/Furniture/Bed/Bed.Bed_C|GettriggerActivated _bed_ref))
        (Default|ActivateHallucination _bed_ref)))
    (:2
      (if (not (Variables|/Game/HorrorEngine/Blueprints/UsableAssets/Electronics/Radio.Radio_C|GetOn%20/%20Off _radio_ref))
        (Default|Open/On _radio_ref false)))
    (:3
      (bind _outactors (Actor|GetAllActorsOfClass "/Game/DemoItems/organ1.organ1_C"))
      (if (== (Utilities|Array|Length _outactors) 0)
        (bind _returnvalue (Game|SpawnActorfromClass "/Game/DemoItems/organ1.organ1_C" (Math|Transform|MakeTransform "564.000000,-352.000000,97.000000" "11.394000,-36.980000,-48.500000" "1.843750,1.000000,1.875000") "AdjustIfPossibleButAlwaysSpawn" 0 0))
        (Default|Activate _returnvalue)
        (bind _outactors_2 (Actor|GetAllActorsOfClass "/Game/HorrorEngine/Blueprints/UsableAssets/Electronics/OldTv.OldTv_C"))
        (for _array_element _outactors_2
          (Default|Open/On _array_element true))))))

(fn ConstructionScript)

(fn GenerateRandomEvent
  (params (Max :type Integer))
  (bind _output_get (Variables|Default|SetCurrentEvent (Math|Random|RandomInteger Max)))
  (Development|PrintString (Utilities|String|Append (Utilities|String|ToString(Integer) _output_get) " is the current event.")))